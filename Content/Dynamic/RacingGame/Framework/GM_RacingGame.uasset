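; Racing game mode that runs a time-trial race against a countdown timer, extended by checkpoints and won at the finish line.
; On BeginPlay it binds every BP_Checkpoint's crossing event by finish-line flag, then starts the race after a delay.
; Checkpoint time is added by re-setting the timer with remaining plus bonus, then playing a HUD animation.
; Timeout loses, finishing clears the timer and wins; countdown and results are only printed strings.
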(event Custom|Game%20Start
  (Development|PrintString "Game has started")
  (bind _returnvalue (Utilities|Time|SetTimerbyEvent (delegate Custom|Lose_OutOfTime) (Variables|Default|GetStartTimerDuration)))
  (Variables|Default|SetTimeRemaining _returnvalue))

(event Custom|Game%20End
  (params (Win :type Boolean))
  (Development|PrintString (Utilities|String|SelectString "You won" "You lost" Win)))

(event Custom|Start%20Countdown
  (Development|PrintString "Hello")
  (Utilities|FlowControl|Delay (Variables|Default|GetStartCountdownDuration))
  (CallFunction|GameStart))

(event Custom|Lose_OutOfTime
  (CallFunction|GameEnd false))

(event Custom|Win_CrossTheFinishLine
  (Utilities|Time|ClearandInvalidateTimerbyHandle (Variables|Default|GetTimeRemaining))
  (CallFunction|GameEnd true))

(event Custom|CrossedACheckpoint
  (params (TimeToAdd :type Integer))
  (CallFunction|AddTimetoTimer TimeToAdd))

(event EventBeginPlay
  (Utilities|FlowControl|Sequence
    (:then_0
      (bind _outactors (Actor|GetAllActorsOfClass "/Game/Dynamic/RacingGame/Checkpoints/BP_Checkpoint.BP_Checkpoint_C"))
      (for _array_element _outactors
        (if (Variables|/Game/Dynamic/RacingGame/Checkpoints/BP_Checkpoint.BP_Checkpoint_C|GetIsFinishLine _array_element)
          (EventDispatchers|BindEventtoOnCheckpointCrossed _array_element (EventDispatchers|CreateEvent :!event Custom|Win_CrossTheFinishLine))
          (else
            (EventDispatchers|BindEventtoOnCheckpointCrossedwithTime _array_element (EventDispatchers|CreateEvent :!event Custom|CrossedACheckpoint))))))
    (:then_1
      (CallFunction|StartCountdown))))

(event EventTick
  (params (DeltaSeconds :type Float%20%28single-precision%29)))

(fn ConstructionScript)

(fn AddTimetoTimer
  (params (TimeToAdd :type Integer))
  (bind _returnvalue (Utilities|Time|SetTimerbyEvent (EventDispatchers|CreateEvent :!event Custom|Lose_OutOfTime) (+ (Utilities|Time|GetTimerRemainingTimebyHandle (Variables|Default|GetTimeRemaining)) TimeToAdd)))
  (Variables|Default|SetTimeRemaining _returnvalue)
  (bind _asvehicle_player_controller (Utilities|Casting|CastToVehiclePlayerController (Game|GetPlayerController 0)))
  (Default|PlayAddedTimeAnim (Variables|/Game/Dynamic/VehicleTemplate/Blueprints/VehiclePlayerController.VehiclePlayerController_C|GetVehicleHud _asvehicle_player_controller)))